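; Menu game mode that tracks the players connected to a multiplayer lobby and keeps their lobby views in sync.
; New players on the Lobby Menu map are stored as shooter menu controllers, then told to create the lobby menu and run initial setup.
; UpdateLobby rebuilds the profile list and pushes names or the selected level to every controller.
; Logouts remove the controller and refresh player names.
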(event `self.K2_OnLogout`
  (params (ExitingController :type "Controller Object Reference"))
  (bind _asbp_shooter_menu_controller (cast `/Game/FrameWork/BP_ShooterMenuController` ExitingController))
  (`KismetArrayLibrary.Array_RemoveItem` (`self.All_ConnectedPlayers`) _asbp_shooter_menu_controller)
  (`self.UpdateLobby` true))

(event `self.HandleStartingNewPlayer`
  (params (NewPlayer :type "PlayerController Object Reference"))
  (bind _returnvalue (`GameplayStatics.GetCurrentLevelName` true))
  (switch `string` _returnvalue
    (:`LobbyMenu_Map`
      (bind _asbp_shooter_menu_controller (cast `/Game/FrameWork/BP_ShooterMenuController` NewPlayer))
      (`KismetArrayLibrary.Array_Add` (`self.All_ConnectedPlayers`) _asbp_shooter_menu_controller)
      (`/Game/FrameWork/BP_ShooterMenuController.CreateLobbyMenu` _asbp_shooter_menu_controller)
      (`/Game/FrameWork/BP_ShooterMenuController.Initial_Setup` _asbp_shooter_menu_controller))))

(event `UpdateLobby`
  (params (PlayerNames :type Boolean) (LevelSelection :type Boolean))
  (if PlayerNames
    (`KismetArrayLibrary.Array_Clear` (`self.All_PlayerProfiles`))
    (for _array_element (`self.All_ConnectedPlayers`)
      (`KismetArrayLibrary.Array_Add` (`self.All_PlayerProfiles`) (`/Game/FrameWork/BP_ShooterMenuController.PlayerProfileInfo` _array_element))))
  (for _array_element_2 (`self.All_ConnectedPlayers`)
    (if PlayerNames
      (`/Game/FrameWork/BP_ShooterMenuController.UpdatePlayerNames` _array_element_2 (`self.All_PlayerProfiles`)))
    (if LevelSelection
      (`/Game/FrameWork/BP_ShooterMenuController.UpdateLevelSelection` _array_element_2 (`self.SelectedLevelName`)))))

(fn `UserConstructionScript`)